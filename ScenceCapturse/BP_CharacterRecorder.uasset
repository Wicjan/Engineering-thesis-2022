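; BP_CharacterRecorder is a scene-capture stand-in for the player character that mirrors equipped gear on its own skeletal mesh.
; On BeginPlay it passes itself to BP_HeroCharacter, and its equip and unequip events call AttachIteam and UnAttachIteam.
; Each slot spawns a collision-free armor or weapon actor snapped to the socket named in its item info.
; Slots replace their previous actor, except Feet, which destroys the Legs item instead.
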(event EventBeginPlay
  (bind _asbp_hero_character (Utilities|Casting|CastToBP_HeroCharacter (Game|GetPlayerCharacter 0)))
  (Class|BPIRecorderComm|PassReference(Message) _asbp_hero_character self))

(event EventEquitIteam
  (params (ItemInfo :type Str%20Item%20Info%20Structure))
  (CallFunction|AttachIteam ItemInfo))

(event EventUnEquitIteam
  (params (ItemInfo :type Str%20Item%20Info%20Structure))
  (CallFunction|UnAttachIteam ItemInfo))

(fn ConstructionScript)

(fn UnAttachIteam
  (params (IteamInfo :type Str%20Item%20Info%20Structure))
  (switch Utilities|FlowControl|Switch|SwitchonE_SlotType (.ItemSlot (Utilities|Struct|BreakStr_ItemInfo IteamInfo))
    (:NewEnumerator1
      (Actor|DestroyActor (Variables|Default|GetHeadIteam)))
    (:NewEnumerator2
      (Actor|DestroyActor (Variables|Default|GetTorsoIteam)))
    (:NewEnumerator3
      (Actor|DestroyActor (Variables|Default|GetArmsIteam)))
    (:NewEnumerator10
      (Actor|DestroyActor (Variables|Default|GetLegsIteam)))
    (:NewEnumerator4
      (Actor|DestroyActor (Variables|Default|GetFeetIteam)))
    (:NewEnumerator5
      (Actor|DestroyActor (Variables|Default|GetPrimaryRightHandIteam)))
    (:NewEnumerator6
      (Actor|DestroyActor (Variables|Default|GetPrimaryLeftHandIteam)))
    (:NewEnumerator7
      (Actor|DestroyActor (Variables|Default|GetSecondaryRightHandIteam)))
    (:NewEnumerator8
      (Actor|DestroyActor (Variables|Default|GetSecondaryLeftHandIteam)))
    (:NewEnumerator9
      (Actor|DestroyActor (Variables|Default|GetAmuletIteam)))))

(fn AttachIteam
  (params (IteamInfo :type Str%20Item%20Info%20Structure))
  (bind (_itemtype _itemname _itemimage _itemclass _itemindex _itemslot) (Utilities|Struct|BreakStr_ItemInfo IteamInfo))
  (switch Utilities|FlowControl|Switch|SwitchonE_SlotType _itemslot
    (:NewEnumerator1
      (Utilities|IsValid (Variables|Default|GetHeadIteam)
        (:Is%20Valid
          (Actor|DestroyActor (Variables|Default|GetHeadIteam)))
        (:Is%20Not%20Valid
          _))
      (bind _returnvalue (Game|SpawnActorfromClass _itemclass (Transformation|GetActorTransform) "AlwaysSpawn" 0 0))
      (bind _output_get (Variables|Default|SetHeadIteam _returnvalue))
      (bind _asbp_base_armor (Utilities|Casting|CastToBP_BaseArmor _output_get))
      (Transformation|AttachComponentToComponent _asbp_base_armor (Variables|Default|GetSkeletalMesh) (Utilities|Struct|BreakStr_ArmorInfo (Variables|/Game/prototyp/Interactabels/Armor/BP_BaseArmor.BP_BaseArmor_C|GetArmorInfo _asbp_base_armor)) "SnapToTarget" "SnapToTarget" "SnapToTarget" true)
      (Collision|SetActorEnableCollision _asbp_base_armor false))
    (:NewEnumerator2
      (Utilities|IsValid (Variables|Default|GetTorsoIteam)
        (:Is%20Valid
          (Actor|DestroyActor (Variables|Default|GetTorsoIteam)))
        (:Is%20Not%20Valid
          _))
      (bind _returnvalue_2 (Game|SpawnActorfromClass _itemclass (Transformation|GetActorTransform) "AlwaysSpawn" 0 0))
      (bind _output_get_2 (Variables|Default|SetTorsoIteam _returnvalue_2))
      (bind _asbp_base_armor_2 (Utilities|Casting|CastToBP_BaseArmor _output_get_2))
      (Transformation|AttachComponentToComponent _asbp_base_armor_2 (Variables|Default|GetSkeletalMesh) (Utilities|Struct|BreakStr_ArmorInfo (Variables|/Game/prototyp/Interactabels/Armor/BP_BaseArmor.BP_BaseArmor_C|GetArmorInfo _asbp_base_armor_2)) "SnapToTarget" "SnapToTarget" "SnapToTarget" true)
      (Collision|SetActorEnableCollision _asbp_base_armor_2 false))
    (:NewEnumerator3
      (Utilities|IsValid (Variables|Default|GetArmsIteam)
        (:Is%20Valid
          (Actor|DestroyActor (Variables|Default|GetArmsIteam)))
        (:Is%20Not%20Valid
          _))
      (bind _returnvalue_3 (Game|SpawnActorfromClass _itemclass (Transformation|GetActorTransform) "AlwaysSpawn" 0 0))
      (bind _output_get_3 (Variables|Default|SetArmsIteam _returnvalue_3))
      (bind _asbp_base_armor_3 (Utilities|Casting|CastToBP_BaseArmor _output_get_3))
      (Transformation|AttachComponentToComponent _asbp_base_armor_3 (Variables|Default|GetSkeletalMesh) (Utilities|Struct|BreakStr_ArmorInfo (Variables|/Game/prototyp/Interactabels/Armor/BP_BaseArmor.BP_BaseArmor_C|GetArmorInfo _asbp_base_armor_3)) "SnapToTarget" "SnapToTarget" "SnapToTarget" true)
      (Collision|SetActorEnableCollision _asbp_base_armor_3 false))
    (:NewEnumerator10
      (Utilities|IsValid (Variables|Default|GetLegsIteam)
        (:Is%20Valid
          (Actor|DestroyActor (Variables|Default|GetLegsIteam)))
        (:Is%20Not%20Valid
          _))
      (bind _returnvalue_4 (Game|SpawnActorfromClass _itemclass (Transformation|GetActorTransform) "AlwaysSpawn" 0 0))
      (bind _output_get_4 (Variables|Default|SetLegsIteam _returnvalue_4))
      (bind _asbp_base_armor_4 (Utilities|Casting|CastToBP_BaseArmor _output_get_4))
      (Transformation|AttachComponentToComponent _asbp_base_armor_4 (Variables|Default|GetSkeletalMesh) (Utilities|Struct|BreakStr_ArmorInfo (Variables|/Game/prototyp/Interactabels/Armor/BP_BaseArmor.BP_BaseArmor_C|GetArmorInfo _asbp_base_armor_4)) "SnapToTarget" "SnapToTarget" "SnapToTarget" true)
      (Collision|SetActorEnableCollision _asbp_base_armor_4 false))
    (:NewEnumerator4
      (Utilities|IsValid (Variables|Default|GetLegsIteam)
        (:Is%20Valid
          (Actor|DestroyActor (Variables|Default|GetLegsIteam)))
        (:Is%20Not%20Valid
          _))
      (bind _returnvalue_5 (Game|SpawnActorfromClass _itemclass (Transformation|GetActorTransform) "AlwaysSpawn" 0 0))
      (bind _output_get_5 (Variables|Default|SetFeetIteam _returnvalue_5))
      (bind _asbp_base_armor_5 (Utilities|Casting|CastToBP_BaseArmor _output_get_5))
      (Transformation|AttachComponentToComponent _asbp_base_armor_5 (Variables|Default|GetSkeletalMesh) (Utilities|Struct|BreakStr_ArmorInfo (Variables|/Game/prototyp/Interactabels/Armor/BP_BaseArmor.BP_BaseArmor_C|GetArmorInfo _asbp_base_armor_5)) "SnapToTarget" "SnapToTarget" "SnapToTarget" true)
      (Collision|SetActorEnableCollision _asbp_base_armor_5 false))
    (:NewEnumerator5
      (Utilities|IsValid (Variables|Default|GetPrimaryRightHandIteam)
        (:Is%20Valid
          (Actor|DestroyActor (Variables|Default|GetPrimaryRightHandIteam)))
        (:Is%20Not%20Valid
          _))
      (bind _returnvalue_6 (Game|SpawnActorfromClass _itemclass (Transformation|GetActorTransform) "AlwaysSpawn" 0 0))
      (bind _output_get_6 (Variables|Default|SetPrimaryRightHandIteam _returnvalue_6))
      (bind _asbp_base_weapon (Utilities|Casting|CastToBP_BaseWeapon _output_get_6))
      (Transformation|AttachComponentToComponent _asbp_base_weapon (Variables|Default|GetSkeletalMesh) (Utilities|Struct|BreakStr_WeaponInfo (Variables|/Game/prototyp/Interactabels/Weapons/BP_BaseWeapon.BP_BaseWeapon_C|GetWeaponInfo _asbp_base_weapon)) "SnapToTarget" "SnapToTarget" "SnapToTarget" true)
      (Collision|SetActorEnableCollision _asbp_base_weapon false))
    (:NewEnumerator6
      (Utilities|IsValid (Variables|Default|GetPrimaryLeftHandIteam)
        (:Is%20Valid
          (Actor|DestroyActor (Variables|Default|GetPrimaryLeftHandIteam)))
        (:Is%20Not%20Valid
          _))
      (bind _returnvalue_7 (Game|SpawnActorfromClass _itemclass (Transformation|GetActorTransform) "AlwaysSpawn" 0 0))
      (bind _output_get_7 (Variables|Default|SetPrimaryLeftHandIteam _returnvalue_7))
      (bind _asbp_base_weapon_2 (Utilities|Casting|CastToBP_BaseWeapon _output_get_7)
        (:then
          (Transformation|AttachComponentToComponent _asbp_base_weapon_2 (Variables|Default|GetSkeletalMesh) (Utilities|Struct|BreakStr_WeaponInfo (Variables|/Game/prototyp/Interactabels/Weapons/BP_BaseWeapon.BP_BaseWeapon_C|GetWeaponInfo _asbp_base_weapon_2)) "SnapToTarget" "SnapToTarget" "SnapToTarget" true)
          (Collision|SetActorEnableCollision _asbp_base_weapon_2 false))
        (:CastFailed
          (bind _asbp_base_armor_6 (Utilities|Casting|CastToBP_BaseArmor _output_get_7))
          (Transformation|AttachComponentToComponent _asbp_base_armor_6 (Variables|Default|GetSkeletalMesh) (Utilities|Struct|BreakStr_ArmorInfo (Variables|/Game/prototyp/Interactabels/Armor/BP_BaseArmor.BP_BaseArmor_C|GetArmorInfo _asbp_base_armor_6)) "SnapToTarget" "SnapToTarget" "SnapToTarget" true)
          (Collision|SetActorEnableCollision _asbp_base_armor_6 false))))
    (:NewEnumerator7
      (Utilities|IsValid (Variables|Default|GetSecondaryRightHandIteam)
        (:Is%20Valid
          (Actor|DestroyActor (Variables|Default|GetSecondaryRightHandIteam)))
        (:Is%20Not%20Valid
          _))
      (bind _returnvalue_8 (Game|SpawnActorfromClass _itemclass (Transformation|GetActorTransform) "AlwaysSpawn" 0 0))
      (bind _output_get_8 (Variables|Default|SetSecondaryRightHandIteam _returnvalue_8))
      (bind _asbp_base_weapon_3 (Utilities|Casting|CastToBP_BaseWeapon _output_get_8))
      (Transformation|AttachComponentToComponent _asbp_base_weapon_3 (Variables|Default|GetSkeletalMesh) (Utilities|Struct|BreakStr_WeaponInfo (Variables|/Game/prototyp/Interactabels/Weapons/BP_BaseWeapon.BP_BaseWeapon_C|GetWeaponInfo _asbp_base_weapon_3)) "SnapToTarget" "SnapToTarget" "SnapToTarget" true)
      (Collision|SetActorEnableCollision _asbp_base_weapon_3 false))
    (:NewEnumerator8
      (Utilities|IsValid (Variables|Default|GetSecondaryLeftHandIteam)
        (:Is%20Valid
          (Actor|DestroyActor (Variables|Default|GetSecondaryLeftHandIteam)))
        (:Is%20Not%20Valid
          _))
      (bind _returnvalue_9 (Game|SpawnActorfromClass _itemclass (Transformation|GetActorTransform) "AlwaysSpawn" 0 0))
      (bind _output_get_9 (Variables|Default|SetSecondaryLeftHandIteam _returnvalue_9))
      (bind _asbp_base_weapon_4 (Utilities|Casting|CastToBP_BaseWeapon _output_get_9)
        (:then
          (Transformation|AttachComponentToComponent _asbp_base_weapon_4 (Variables|Default|GetSkeletalMesh) (Utilities|Struct|BreakStr_WeaponInfo (Variables|/Game/prototyp/Interactabels/Weapons/BP_BaseWeapon.BP_BaseWeapon_C|GetWeaponInfo _asbp_base_weapon_4)) "SnapToTarget" "SnapToTarget" "SnapToTarget" true)
          (Collision|SetActorEnableCollision _asbp_base_weapon_4 false))
        (:CastFailed
          (bind _asbp_base_armor_7 (Utilities|Casting|CastToBP_BaseArmor _output_get_9))
          (Transformation|AttachComponentToComponent _asbp_base_armor_7 (Variables|Default|GetSkeletalMesh) (Utilities|Struct|BreakStr_ArmorInfo (Variables|/Game/prototyp/Interactabels/Armor/BP_BaseArmor.BP_BaseArmor_C|GetArmorInfo _asbp_base_armor_7)) "SnapToTarget" "SnapToTarget" "SnapToTarget" true)
          (Collision|SetActorEnableCollision _asbp_base_armor_7 false))))
    (:NewEnumerator9
      (Utilities|IsValid (Variables|Default|GetAmuletIteam)
        (:Is%20Valid
          (Actor|DestroyActor (Variables|Default|GetAmuletIteam)))
        (:Is%20Not%20Valid
          _))
      (bind _returnvalue_10 (Game|SpawnActorfromClass _itemclass (Transformation|GetActorTransform) "AlwaysSpawn" 0 0))
      (bind _output_get_10 (Variables|Default|SetAmuletIteam _returnvalue_10))
      (bind _asbp_base_armor_8 (Utilities|Casting|CastToBP_BaseArmor _output_get_10))
      (Transformation|AttachComponentToComponent _asbp_base_armor_8 (Variables|Default|GetSkeletalMesh) (Utilities|Struct|BreakStr_ArmorInfo (Variables|/Game/prototyp/Interactabels/Armor/BP_BaseArmor.BP_BaseArmor_C|GetArmorInfo _asbp_base_armor_8)) "SnapToTarget" "SnapToTarget" "SnapToTarget" true)
      (Collision|SetActorEnableCollision _asbp_base_armor_8 false))))