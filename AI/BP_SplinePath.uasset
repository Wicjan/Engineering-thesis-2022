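; BP_SplinePath is an actor that moves a static mesh along a spline in a repeating loop.
; A timeline track drives a lerp over the spline length, and the resulting world-space location is applied to the mesh each update.
; The timeline starts on BeginPlay and restarts from the beginning after a short delay when it finishes.
; Pause and Continue events stop and resume the motion.
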(event Custom|Pause
  (bind _newtrack_0 (Timeline|Timeline_0 Stop)
    (:Update
      (Variables|Default|SetLocation (Spline|GetLocationatDistanceAlongSpline (Variables|Default|GetSpline) (Math|Float|Lerp 0.0 (Spline|GetSplineLength (Variables|Default|GetSpline)) _newtrack_0) "World"))
      (Transformation|SetWorldLocation (Variables|Default|GetStaticMesh) (Spline|GetLocationatDistanceAlongSpline (Variables|Default|GetSpline) (Math|Float|Lerp 0.0 (Spline|GetSplineLength (Variables|Default|GetSpline)) _newtrack_0) "World") false false))
    (:Finished
      (Utilities|FlowControl|Delay 0.2)
      (Timeline|Timeline_0 PlayFromStart))))

(event Custom|Continue
  (bind _newtrack_0 (Timeline|Timeline_0 Play)
    (:Update
      (Variables|Default|SetLocation (Spline|GetLocationatDistanceAlongSpline (Variables|Default|GetSpline) (Math|Float|Lerp 0.0 (Spline|GetSplineLength (Variables|Default|GetSpline)) _newtrack_0) "World"))
      (Transformation|SetWorldLocation (Variables|Default|GetStaticMesh) (Spline|GetLocationatDistanceAlongSpline (Variables|Default|GetSpline) (Math|Float|Lerp 0.0 (Spline|GetSplineLength (Variables|Default|GetSpline)) _newtrack_0) "World") false false))
    (:Finished
      (Utilities|FlowControl|Delay 0.2)
      (Timeline|Timeline_0 PlayFromStart))))

(event EventBeginPlay
  (bind _newtrack_0 (Timeline|Timeline_0 PlayFromStart)
    (:Update
      (Variables|Default|SetLocation (Spline|GetLocationatDistanceAlongSpline (Variables|Default|GetSpline) (Math|Float|Lerp 0.0 (Spline|GetSplineLength (Variables|Default|GetSpline)) _newtrack_0) "World"))
      (Transformation|SetWorldLocation (Variables|Default|GetStaticMesh) (Spline|GetLocationatDistanceAlongSpline (Variables|Default|GetSpline) (Math|Float|Lerp 0.0 (Spline|GetSplineLength (Variables|Default|GetSpline)) _newtrack_0) "World") false false))
    (:Finished
      (Utilities|FlowControl|Delay 0.2)
      (Timeline|Timeline_0 PlayFromStart))))

(fn ConstructionScript)