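; Enemy character Blueprint that wanders, takes punch damage and attacks the hero with a sword.
; BeginPlay attaches the sword mesh to a hand socket and caches the hero reference; MoveToRandomLocation loops through random nearby navigable points.
; AttackPlayer plays a slash montage, then runs a debug-drawn forward sphere trace that damages the hero on any hit.
; Overlapping an attacking, unarmed hero applies that hero's attack damage to the enemy.
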(event Custom|MoveToRandomLocation
  (AI|AIMoveTo self (.RandomLocation (Class|NavigationSystemV1|GetRandomPointinNavigableRadius (Transformation|GetActorLocation) 3e+02 0 0)) 0 5.0 false
    (:OnSuccess
      (Utilities|FlowControl|Delay 1.0)
      (CallFunction|MovetoRandomLocation))))

(event Custom|AttackPlayer
  (if (not (Variables|Default|GetIsAttacking?))
    (Variables|Default|SetIsAttacking? true)
    (Animation|PlayAnimMontage "/Game/prototyp/Animation/Sword_And_Shield_Slash_Montage.Sword_And_Shield_Slash_Montage" 1.0 "None")
    (Utilities|FlowControl|Delay 1.0)
    (CallFunction|CreateDamageSphere)
    (Variables|Default|SetIsAttacking? false)))

(event Collision|EventActorBeginOverlap
  (params (OtherActor :type Actor%20Object%20Reference))
  ;[1 1 1] While hero punch
  (bind _asbp_hero_character (Utilities|Casting|CastToBP_HeroCharacter OtherActor))
  (if (not (Variables|/Game/prototyp/BP_HeroCharacter.BP_HeroCharacter_C|GetHasWeaponAttached _asbp_hero_character))
    (if (Variables|/Game/prototyp/BP_HeroCharacter.BP_HeroCharacter_C|GetIsAttacking? _asbp_hero_character)
      (Utilities|FlowControl|DoOnce false :!label _label
        (:Completed
          (Game|Damage|ApplyDamage self (Variables|/Game/prototyp/BP_HeroCharacter.BP_HeroCharacter_C|GetAttack_Damage _asbp_hero_character) 0 0)
          (goto _label Reset))))))

(event EventBeginPlay
  (Transformation|AttachComponentToComponent (Variables|Default|GetStaticMesh) (Variables|Character|GetMesh) "EnemySwordSocket" "SnapToTarget" "SnapToTarget" "SnapToTarget" true)
  (bind _asbp_enemy_character (Utilities|Casting|CastToBP_EnemyCharacter self))
  (Variables|Default|SetEnemyReference _asbp_enemy_character)
  (bind _asbp_hero_character (Utilities|Casting|CastToBP_HeroCharacter (Game|GetPlayerCharacter 0)))
  (Variables|Default|SetCharacterReference _asbp_hero_character))

(fn ConstructionScript)

(fn CreateDamageSphere
  (bind _enemyreference (Variables|Default|GetEnemyReference))
  (bind _returnvalue (Transformation|GetActorLocation _enemyreference))
  (bind _returnvalue_2 (Collision|MultiSphereTraceByChannel _returnvalue (+ _returnvalue (* (Transformation|GetActorForwardVector _enemyreference) 2.5e+02)) 0.0 "TraceTypeQuery2" false (Utilities|Array|MakeArray _enemyreference) "ForDuration"))
  (if _returnvalue_2
    (Game|Damage|ApplyDamage (Variables|Default|GetCharacterReference) 5.0 0 0)))