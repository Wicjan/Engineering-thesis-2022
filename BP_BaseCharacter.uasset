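; Base character Blueprint that handles health, death and experience-based leveling.
; AnyDamage subtracts health and, while the character survives, plays a hit montage gated by a DoOnce that resets after a short delay.
; At zero health, it awards EXP to player 0's BP_HeroCharacter, ragdolls the mesh, clears IsAlive and calls OnDeath on its BP_PlayerControler, if present.
; AddEXP carries surplus EXP into the next level, scales the requirement with level and grants a skill point.
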(event Game|Damage|EventAnyDamage
  (params (Damage :type Float%20%28single-precision%29) (DamageType :type Damage%20Type%20Object%20Reference) (InstigatedBy :type Controller%20Object%20Reference) (DamageCauser :type Actor%20Object%20Reference))
  (bind _output_get (Variables|Default|SetCurrentHealth (- (Variables|Default|GetCurrentHealth) Damage)))
  (if (<= _output_get 0.0)
    (bind _asbp_hero_character (Utilities|Casting|CastToBP_HeroCharacter (Game|GetPlayerCharacter 0)))
    (CallFunction|AddEXP _asbp_hero_character 5e+01)
    (Physics|SetSimulatePhysics (Variables|Character|GetMesh) true)
    (Variables|Default|SetIsAlive? false)
    (bind _asbp_player_controler (Utilities|Casting|CastToBP_PlayerControler (Pawn|GetController)))
    (Default|OnDeath _asbp_player_controler)
    (else
      (Utilities|FlowControl|DoOnce false :!label _label
        (:Completed
          (Animation|PlayAnimMontage "/Game/prototyp/Animation/HitToBody.HitToBody" 1.0 "None")
          (Utilities|FlowControl|Delay 0.5)
          (goto _label Reset))))))

(fn ConstructionScript)

(fn AddEXP
  (params (Added%20EXP :type Float%20%28single-precision%29))
  (bind _characterlevel (Variables|Default|GetCharacterLevel))
  (bind _output_get (Variables|Default|SetCurrentEXP (+ Added%20EXP (Variables|Default|GetCurrentEXP))))
  (if (>= _output_get (Variables|Default|GetNeededEXP))
    (Variables|Default|SetCurrentEXP (- _output_get (Variables|Default|GetNeededEXP)))
    (Math|Integer|IncrementInt _characterlevel
      (:%20%20
        (Variables|Default|SetNeededEXP (* _characterlevel 1e+02))
        (CallFunction|AddSkillPoint)))))

(fn AddSkillPoint
  (Math|Integer|IncrementInt (Variables|Default|GetSkillPoints)))