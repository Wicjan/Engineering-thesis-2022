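; BP_BaseWeapon is a base weapon Blueprint that performs the player hero's attack.
; On BeginPlay it caches the player's BP_HeroCharacter.
; Attack runs a multi sphere trace on the Camera channel along the hero's forward vector, ignoring the hero and drawing debug shapes.
; Each hit spawns VFX, plays a sound and applies damage, with range, damage and effects read from WeaponInfo.
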(event Custom|Attack
  (bind _heroreference (Variables|Default|GetHeroReference))
  (bind _weaponinfo (Variables|Default|GetWeaponInfo))
  (bind (_damage _hitvfx _hitsfx) (Utilities|Struct|BreakStr_WeaponInfo _weaponinfo))
  (bind _returnvalue (Transformation|GetActorLocation _heroreference))
  (bind (_outhits _returnvalue_2) (Collision|MultiSphereTraceByChannel _returnvalue (+ _returnvalue (* (Transformation|GetActorForwardVector _heroreference) (.range (Variables|Default|GetWeaponInfo)))) 0.0 "TraceTypeQuery2" false (Utilities|Array|MakeArray _heroreference) "ForDuration"))
  (if _returnvalue_2
    (for _array_element _outhits
      (Effects|SpawnEmitteratLocation _hitvfx (.Location (Collision|BreakHitResult _array_element)))
      (Audio|PlaySoundatLocation _hitsfx (.Location (Collision|BreakHitResult _array_element)) "0, 0, 0" 1.0 1.0 0.0 0 0 0)
      (Game|Damage|ApplyDamage (.HitActor (Collision|BreakHitResult _array_element)) _damage 0 (Variables|Default|GetHeroReference)))))

(event EventBeginPlay
  (bind _asbp_hero_character (Utilities|Casting|CastToBP_HeroCharacter (Game|GetPlayerCharacter 0)))
  (Variables|Default|SetHeroReference _asbp_hero_character))

(event Collision|EventActorBeginOverlap
  (params (OtherActor :type Actor%20Object%20Reference)))

(event EventTick
  (params (DeltaSeconds :type Float%20%28single-precision%29)))

(fn ConstructionScript
  (|CallParentFunction))