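; BP_BaseItem is a base pickup item that an instigator collects by interacting with it.
; Its construction script writes the item's own class into the IteamInfo struct, keeping the other fields intact.
; On interaction, it checks the instigator for inventory space, then passes IteamInfo through PickUpMessage and destroys itself.
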(event EventInteracion
  (params (Instigator :type BP%20Hero%20Character%20Object%20Reference))
  (if (Default|CheckSpaceinInventory Instigator)
    (Class|BPIInteract|PickUp(Message) Instigator (Variables|Default|GetIteamInfo))
    (Actor|DestroyActor)))

(fn ConstructionScript
  (|CallParentFunction)
  (Variables|Default|SetIteamInfo (Utilities|Struct|MakeStr_ItemInfo (.itemtype (Variables|Default|GetIteamInfo)) (.itemname (Variables|Default|GetIteamInfo)) (.itemimage (Variables|Default|GetIteamInfo)) (Utilities|GetClass self) (.itemindex (Variables|Default|GetIteamInfo)) (.itemslot (Variables|Default|GetIteamInfo)) (.itemvalue (Variables|Default|GetIteamInfo)))))