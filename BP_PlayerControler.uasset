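; Player controller Blueprint that handles the player's death sequence and restarts the game afterward.
; On death it unpossesses the pawn, fades the camera to black and shows a death screen widget.
; After a short delay it removes the widget and asks the ThirdPersonGameMode to restart the game.
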(event Custom|OnDeath
  (Pawn|UnPossess)
  (CameraFades|StartCameraFade (Variables|Default|GetPlayerCameraManager) 0.0 1.0 2.0 "(R=0.000000,G=0.000000,B=0.000000,A=1.000000)" false false)
  (bind _returnvalue (UserInterface|CreateWidget "/Game/prototyp/Widgets/WI_DeadScreen.WI_DeadScreen_C" self))
  (UserInterface|Viewport|AddtoViewport _returnvalue 0)
  (Utilities|FlowControl|Delay 2.0)
  (Widget|RemovefromParent _returnvalue)
  (bind _asthird_person_game_mode (Utilities|Casting|CastToThirdPersonGameMode (Game|GetGameMode)))
  (Class|GameMode|RestartGame _asthird_person_game_mode))

(event EventBeginPlay)

(event EventTick
  (params (DeltaSeconds :type Float%20%28single-precision%29)))

(fn ConstructionScript)